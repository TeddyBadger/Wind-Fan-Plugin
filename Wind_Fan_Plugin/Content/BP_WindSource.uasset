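; BP_WindSource is a placeable wind emitter that pushes or pulls movable actors inside a capsule area while switched on.
; Construction sizes the capsule from Length, takes Direction from the cylinder's up vector and fits the Niagara effect to both shapes.
; Overlaps track actors tagged "Movable".
; Tick applies force through their AC_Movable component, boosting characters via movement component and accelerating other primitives independent of mass.
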(event `self.WindArea.OnComponentBeginOverlap`
  (params (OverlappedComponent :type "PrimitiveComponent Object Reference") (OtherActor :type "Actor Object Reference") (OtherComp :type "PrimitiveComponent Object Reference") (OtherBodyIndex :type Integer) (bFromSweep :type Boolean) (SweepResult :type "HitResult Structure (by ref)"))
  ; This part makes sure only actors with "AC_Movable" in them can be affected:
  (if (`self.ActorHasTag` OtherActor "Movable")
    (`KismetArrayLibrary.Array_AddUnique` (`self.OverlappingActors`) OtherActor)))

(event `self.WindArea.OnComponentEndOverlap`
  (params (OverlappedComponent :type "PrimitiveComponent Object Reference") (OtherActor :type "Actor Object Reference") (OtherComp :type "PrimitiveComponent Object Reference") (OtherBodyIndex :type Integer))
  ; This part makes sure only actors with "AC_Movable" in them can be affected:
  (if (`self.ActorHasTag` OtherActor "Movable")
    (`KismetArrayLibrary.Array_RemoveItem` (`self.OverlappingActors`) OtherActor)))

(event `self.ReceiveBeginPlay`
  ; This controls the wind particle effects:
  (`NiagaraComponent.SetVariableVec3` (`self.NS_Wind`) "Velocity" (`self.Direction`))
  (if (`self.On?`)
    (`ActorComponent.Activate` (`self.NS_Wind`) false)
    (else
      (`ActorComponent.Deactivate` (`self.NS_Wind`)))))

(event `self.ReceiveTick`
  (params (DeltaSeconds :type "Float (single-precision)"))
  (bind _returnvalue (* (`self.Direction`) (`self.Strength`)))
  ; This whole section is the part that actually causes the object to be pushed:
  (if (`self.On?`)
    (`ActorComponent.Activate` (`self.NS_Wind`) false)
    (for _array_element (`self.OverlappingActors`)
      (bind _returnvalue_2 (`self.GetComponentByClass` _array_element "/Game/Base/Blueprints/Actors/Parents/AC_Movable.AC_Movable_C"))
      ;; Due to the script being a bit different for pushing the player, a branch is needed to check if the actor trying to be affected is the player or not. If it is, this part affects the pushing or pulling of the player:
      (if (`/Game/Base/Blueprints/Actors/Parents/AC_Movable.IsCharacter?` _returnvalue_2)
        (if (`self.Push?`)
          (bind _charmovementcomponent (`/Game/Base/Blueprints/Actors/Parents/AC_Movable.CharMovementComponent` _returnvalue_2))
          (`CharacterMovementComponent.AddForce` _charmovementcomponent (* (`self.Direction`) (`self.Strength`) (`self.CharExtraStrength`)))
          (else
            (`CharacterMovementComponent.AddForce` _charmovementcomponent (* (`self.Direction`) (`self.Strength`) (`self.Negative`) (`self.CharExtraStrength`)))))
        (else
          (bind (_primitivecomponent _isvalid) (`/Game/Base/Blueprints/Actors/Parents/AC_Movable.GetPrimative` _returnvalue_2))
          ;; If the actor being affected is NOT the player, then this part handles that interaction:
          (if _isvalid
            (if (`self.Push?`)
              (`PrimitiveComponent.AddForce` _primitivecomponent _returnvalue "None" true)
              (else
                (`PrimitiveComponent.AddForce` _primitivecomponent (* _returnvalue (`self.Negative`)) "None" true)))))))
    (else
      (`ActorComponent.Deactivate` (`self.NS_Wind`)))))

(fn `UserConstructionScript`
  (bind _relativescale3d_x (`KismetMathLibrary.BreakVector` (`SceneComponent.RelativeScale3D` (`self.Cylinder`))))
  (`CapsuleComponent.SetCapsuleHalfHeight` (`self.WindArea`) (`self.Length`) true)
  (set `self.Direction` (`SceneComponent.GetUpVector` (`self.Cylinder`)))
  (`NiagaraComponent.SetNiagaraVariableFloat` (`self.NS_Wind`) "Height" (* (`CapsuleComponent.CapsuleHalfHeight` (`self.WindArea`)) 0.8))
  (`NiagaraComponent.SetNiagaraVariableFloat` (`self.NS_Wind`) "Radius" (* _relativescale3d_x 80.0)))