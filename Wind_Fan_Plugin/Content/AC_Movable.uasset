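; AC_Movable is an actor component that marks its owner as affected by movement effects by adding the "Movable" tag on BeginPlay.
; It then looks up the configurable ComponentToLookFor class on the owner, caching a PrimitiveComponent, or a CharacterMovementComponent with IsCharacter set.
; If neither cast succeeds it prints an error.
; GetPrimative returns the cached primitive with a validity flag, without covering the character movement case.
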(event `self.ReceiveBeginPlay`
  ; This takes the actor it is attached to and gives it the "Movable" tag which will allow it to be affected:
  (`KismetArrayLibrary.Array_Add` (`Actor.Tags` (`self.GetOwner`)) "Movable")
  (`self.SetPrimative`))

(fn `GetPrimative`
  (returns (PrimitiveComponent :type "PrimitiveComponent Object Reference") (IsValid :type Boolean))
  ; This simply gets the primative component and checks if it is a valid primative or not:
  (bind _primitivecomponent (`self.PrimitiveComponent`)
    (:`then`
      (return _primitivecomponent true))
    (:`else`
      (return null false))))

(fn `SetPrimative`
  (bind _returnvalue (`Actor.GetComponentByClass` (`self.GetOwner`) (`self.ComponentToLookFor`)))
  ; This then sets what part of the actor is the primative component, otherwise errors occur when trying to push the player:
  (bind _asprimitive_component (cast `PrimitiveComponent` _returnvalue)
    (:`then`
      (set `self.PrimitiveComponent` _asprimitive_component)
      (return))
    (:`CastFailed`
      (bind _ascharacter_movement_component (cast `CharacterMovementComponent` _returnvalue)
        (:`then`
          (set `self.IsCharacter?` true)
          (set `self.CharMovementComponent` _ascharacter_movement_component)
          (return))
        (:`CastFailed`
          (`KismetSystemLibrary.PrintString` "Wrong Component Class Selected Or Not Found"))))))